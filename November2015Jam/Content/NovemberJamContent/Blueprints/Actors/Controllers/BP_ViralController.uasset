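; BP_ViralController is an AI controller that sends its possessed viral pawn toward the heart actor.
; BeginPlay caches the heart reference from BP_GameInstance, printing debug output on its validity or on cast failure.
; OnPossess calls MovePawnToTarget immediately and on a looping one-second timer, re-issuing MoveToLocation at the heart's current location.
; The BB_Viral blackboard and BT_Viral behavior tree setup is disconnected and never runs.
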(event `self.ReceiveBeginPlay`
  (bind _asbp_game_instance (cast `/Game/NovemberJamContent/Blueprints/GameData/BP_GameInstance` (`GameplayStatics.GetGameInstance`))
    (:`then`
      (bind _bp_heartref (`/Game/NovemberJamContent/Blueprints/GameData/BP_GameInstance.BP_HeartRef` _asbp_game_instance))
      (set `self.HeartRef` _bp_heartref)
      (`KismetSystemLibrary.PrintString` (`KismetStringLibrary.Conv_BoolToString` (`KismetSystemLibrary.IsValid` _bp_heartref))))
    (:`CastFailed`
      (`KismetSystemLibrary.PrintString` "game instance cast failed"))))

(event `self.OnPossess`
  (params (PossessedPawn :type "Pawn Object Reference"))
  (`KismetSystemLibrary.K2_SetTimer` null "movePawnToTarget" 1.0 true)
  (`self.movePawnToTarget`))

(event `self.ReceiveTick`
  (params (DeltaSeconds :type "Float (single-precision)")))

(fn `movePawnToTarget`
  (`self.MoveToLocation` (`self.K2_GetActorLocation` (`self.HeartRef`))))

(fn `UserConstructionScript`)