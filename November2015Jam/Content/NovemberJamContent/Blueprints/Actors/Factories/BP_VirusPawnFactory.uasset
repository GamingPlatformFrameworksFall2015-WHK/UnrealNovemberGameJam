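; BP_VirusPawnFactory is a spawner actor that produces viral organisms on a repeating timer.
; Tick accumulates delta time and, each time it reaches the loop interval, subtracts that interval and always spawns a BP_ViralOrganism at the factory's transform.
; Each new organism receives its HeartTarget from the heart reference held on BP_GameInstance.
; Disconnected AI controller nodes remain in the graph and never run.
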(event `self.ReceiveBeginPlay`)

(event `self.ReceiveActorBeginOverlap`
  (params (OtherActor :type "Actor Object Reference")))

(event `self.ReceiveTick`
  (params (DeltaSeconds :type "Float (single-precision)"))
  (bind _spawnlooptime (`self.SpawnLoopTime`))
  (bind _currentspawntime (`self.CurrentSpawnTime`))
  (bind _output_get (set `self.CurrentSpawnTime` (+ _currentspawntime DeltaSeconds)))
  (if (>= _output_get _spawnlooptime)
    (set `self.CurrentSpawnTime` (- _currentspawntime _spawnlooptime))
    (bind _returnvalue (`|SpawnActorFromClass` "/Game/NovemberJamContent/Blueprints/Actors/Pawns/Characters/BP_ViralOrganism.BP_ViralOrganism_C" (`self.GetTransform` self) "AlwaysSpawn" "OverrideRootScale"))
    (bind _asbp_game_instance (cast `/Game/NovemberJamContent/Blueprints/GameData/BP_GameInstance` (`GameplayStatics.GetGameInstance`)))
    (set `/Game/NovemberJamContent/Blueprints/Actors/Pawns/Characters/BP_ViralOrganism.HeartTarget` (`/Game/NovemberJamContent/Blueprints/GameData/BP_GameInstance.BP_HeartRef` _asbp_game_instance) _returnvalue)))

(fn `UserConstructionScript`)