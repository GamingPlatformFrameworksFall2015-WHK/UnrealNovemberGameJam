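; BP_ViralOrganism is an AI-driven viral organism character that moves toward a target through BP_ViralController.
; On BeginPlay it spawns its own controller, passing HeartTarget as HeartRef, and possesses itself with it.
; A looping half-second timer then calls MovePawnToTarget on that controller, which holds the movement logic.
; The construction script also sets AIControllerClass to BP_ViralController, alongside the manual spawn.
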(event `self.ReceiveBeginPlay`
  (bind _returnvalue (`|SpawnActorFromClass` "/Game/NovemberJamContent/Blueprints/Actors/Controllers/BP_ViralController.BP_ViralController_C" (`self.GetTransform` self) "Undefined" "OverrideRootScale" null (`self.HeartTarget`)))
  (`Controller.Possess` _returnvalue self)
  (`KismetSystemLibrary.K2_SetTimerDelegate` (delegate `MoveToTarget`) 0.5 true))

(event `self.ReceiveActorBeginOverlap`
  (params (OtherActor :type "Actor Object Reference")))

(event `MoveToTarget`
  (bind _returnvalue (`AIBlueprintHelperLibrary.GetAIController` null))
  (bind _asbp_viral_controller (cast `/Game/NovemberJamContent/Blueprints/Actors/Controllers/BP_ViralController` _returnvalue))
  (`/Game/NovemberJamContent/Blueprints/Actors/Controllers/BP_ViralController.movePawnToTarget` _asbp_viral_controller))

(event `self.ReceiveTick`
  (params (DeltaSeconds :type "Float (single-precision)")))

(fn `UserConstructionScript`
  (`parent.UserConstructionScript`)
  (set `self.AIControllerClass` "/Game/NovemberJamContent/Blueprints/Actors/Controllers/BP_ViralController.BP_ViralController_C"))