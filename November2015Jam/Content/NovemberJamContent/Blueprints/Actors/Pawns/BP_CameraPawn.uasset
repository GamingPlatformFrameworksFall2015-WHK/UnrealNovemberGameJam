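; BP_CameraPawn is a camera pawn the player moves around and zooms with a spring arm.
; MoveForward and MoveRight axes feed movement input along vectors built from control-rotation pitch only, with yaw and roll zeroed, so control yaw does not steer movement.
; ZoomIn and ZoomOut presses step the arm length by a set interval, clamped between zoom limits.
; The construction script starts the arm at maximum zoom distance.
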(event `self.ReceiveBeginPlay`)

(event `self.ReceiveActorBeginOverlap`
  (params (OtherActor :type "Actor Object Reference")))

(event `self.ReceiveTick`
  (params (DeltaSeconds :type "Float (single-precision)")))

(event `InputAxis|MoveRight`
  (params (AxisValue :type "Float (single-precision)"))
  (`self.AddMovementInput` (`KismetMathLibrary.GetRightVector` (`KismetMathLibrary.MakeRotator` 0.0 (.pitch (`self.GetControlRotation`)))) AxisValue))

(event `InputAxis|MoveForward`
  (params (AxisValue :type "Float (single-precision)"))
  (`self.AddMovementInput` (`KismetMathLibrary.GetForwardVector` (`KismetMathLibrary.MakeRotator` 0.0 (.pitch (`self.GetControlRotation`)))) AxisValue))

(event `InputAction|ZoomIn`
  (params (Key :type "Key Structure" :default "AnyKey"))
  (bind _springarm (`self.SpringArm`))
  ;[1 1 1] ZoomIn & ZoomOut
  (:`Pressed`
    (set `SpringArmComponent.TargetArmLength` (`KismetMathLibrary.FClamp` (- (`SpringArmComponent.TargetArmLength` _springarm) (`self.ZoomInterval`)) (`self.MinZoom`) (`self.MaxZoom`)) _springarm)))

(event `InputAction|ZoomOut`
  (params (Key :type "Key Structure" :default "AnyKey"))
  (bind _springarm (`self.SpringArm`))
  ;[1 1 1] ZoomIn & ZoomOut
  (:`Pressed`
    (set `SpringArmComponent.TargetArmLength` (`KismetMathLibrary.FClamp` (+ (`SpringArmComponent.TargetArmLength` _springarm) (`self.ZoomInterval`)) (`self.MinZoom`) (`self.MaxZoom`)) _springarm)))

(fn `UserConstructionScript`
  (set `SpringArmComponent.TargetArmLength` (`self.MaxZoom`) (`self.SpringArm`)))